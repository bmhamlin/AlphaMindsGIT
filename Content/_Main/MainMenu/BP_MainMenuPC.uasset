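; Main menu player controller that gathers the local player's identity when the menu starts.
; After a short delay, with Steam present, it reads the player name and avatar into PlayerInfo, saves it through the game instance, triggers its main menu player info message, then fetches friends.
; Avatar success and failure share that path; without Steam, it only sets PlayerName from the platform user name.
; MainMenuPC returns the controller itself.
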(event `self.ReceiveBeginPlay`
  (bind _returnvalue (`GameplayStatics.GetGameInstance`))
  ;[1 1 1] Begin Play : Get player steam name
  (`KismetSystemLibrary.Delay` 0.2)
  (if (`AdvancedSessionsLibrary.HasOnlineSubsystem` "steam")
    (set `self.PlayerName` (`KismetTextLibrary.Conv_StringToText` (`PlayerState.GetPlayerName` (`self.PlayerState`))))
    (bind _returnvalue_2 (`AdvancedSteamFriendsLibrary.GetSteamFriendAvatar` (`AdvancedSessionsLibrary.GetUniqueNetID` self))
      (:`OnSuccess`
        _)
      (:`OnFailure`
        _))
    (bind _structout (setmembers `/Game/_Main/S_PlayerInfo` :`StructRef` (`self.PlayerInfo`) :`Player Name` (`self.PlayerName`) :`Player Image` _returnvalue_2))
    (message `/Game/_Main/INT_GameInstance.SavePlayerInfo` _returnvalue _structout)
    (message `/Game/_Main/INT_GameInstance.Main Menu Player Info` _returnvalue)
    (bind _results (`GetFriendsCallbackProxy.GetAndStoreFriendsList` self)
      (:`then`
        (for _ _results
          _)))
    (else
      (set `self.PlayerName` (`KismetTextLibrary.Conv_StringToText` (`KismetSystemLibrary.GetPlatformUserName`))))))

(fn `MainMenu PC`
  (returns (`Main Menu PC` :type "/Game/_Main/MainMenu/BP_MainMenuPC Object Reference"))
  (return self))

(fn `UserConstructionScript`)